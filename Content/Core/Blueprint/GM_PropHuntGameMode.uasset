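; Game mode for a prop hunt match that picks one random player as the prop, runs a timed round and restarts the map afterwards.
; Once two players join, a short timer triggers the pick, retrying on an invalid result, then swaps that player's pawn for BP_PropCharacter.
; Player controllers receive role, countdown and win-screen widget messages.
; Round timeout gives the prop the win, and ServerTravel reloads ThirdPersonMap.
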(event `self.K2_PostLogin`
  (params (NewPlayer :type "PlayerController Object Reference"))
  (`KismetArrayLibrary.Array_Add` (`self.Players`) NewPlayer)
  (if (`self.HasTheGameStarted?`)
    _
    (elif (>= (`KismetArrayLibrary.Array_Length` (`self.Players`)) 2)
      (`self.StartGameTimer`))))

(event `StartGameTimer`
  (`KismetSystemLibrary.K2_SetTimerDelegate` (delegate `ChoosePropCharacter`) 4.0))

(event `ChoosePropCharacter`
  (bind _players (`self.Players`))
  (bind _prophuntplayer (`self.PropHuntPlayer`))
  (set `self.HasTheGameStarted?` true)
  (bind _output_get (set `self.PropHuntPlayer` (`|GetArrayItem` _players (`KismetMathLibrary.RandomIntegerInRange` 0 (`KismetArrayLibrary.Array_Length` _players)))))
  (`/Engine/EditorBlueprintResources/StandardMacros.IsValid` _output_get
    (:`Is Valid`
      (bind _returnvalue (`|SpawnActorFromClass` "/Game/Core/Blueprint/BP_PropCharacter.BP_PropCharacter_C" (`KismetMathLibrary.MakeTransform` (`self.Spawn Transform Location`)) "Undefined" "MultiplyWithRoot" null null))
      (`self.K2_DestroyActor` (`Controller.K2_GetPawn` _prophuntplayer))
      (`KismetSystemLibrary.Delay` 0.2)
      (`Controller.Possess` _prophuntplayer _returnvalue)
      (message `/Game/Core/Blueprint/Interfaces/BPI_PropHuntController.SetupPropWidget` _prophuntplayer true)
      (for _array_element (`self.Players`)
        (`/Engine/EditorBlueprintResources/StandardMacros.IsValid` _array_element
          (:`Is Valid`
            (message `/Game/Core/Blueprint/Interfaces/BPI_PropHuntController.StartCountDownWidget` _array_element)
            (bind _prophuntplayer_2 (`self.PropHuntPlayer`)
              (:`then`
                (if (!= _prophuntplayer_2 _array_element)
                  (message `/Game/Core/Blueprint/Interfaces/BPI_PropHuntController.SetupPropWidget` _array_element false)))
              (:`else`)))))
      (`self.StartGameLoopTimer`))
    (:`Is Not Valid`
      (`KismetSystemLibrary.Delay` 1.0)
      (`self.ChoosePropCharacter`))))

(event `StartGameLoopTimer`
  (bind _returnvalue (`KismetSystemLibrary.K2_SetTimerDelegate` (delegate `EndGame`) 300.0))
  (set `self.GameLoopTimer` _returnvalue))

(event `EndGame`
  (`self.EndTheGame` true))

(event `/Game/Core/Blueprint/Interfaces/BPI_PropHuntGameMode.EndTheGame`
  (params (`PropWon?` :type Boolean))
  (`KismetSystemLibrary.K2_ClearAndInvalidateTimerHandle` (`self.GameLoopTimer`))
  (set `self.Prop Won?` `PropWon?`)
  (for _array_element (`self.Players`)
    (`/Engine/EditorBlueprintResources/StandardMacros.IsValid` _array_element
      (:`Is Valid`
        (message `/Game/Core/Blueprint/Interfaces/BPI_PropHuntController.ShowWinScreenWidget` _array_element (`self.Prop Won?`)))))
  (`KismetSystemLibrary.K2_SetTimerDelegate` (delegate `StartNextGame`) 3.0))

(event `StartNextGame`
  (`KismetSystemLibrary.ExecuteConsoleCommand` "ServerTravel ThirdPersonMap" null))

(fn `UserConstructionScript`)