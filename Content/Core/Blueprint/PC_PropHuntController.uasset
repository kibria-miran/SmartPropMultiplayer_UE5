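; Player controller for a Prop Hunt game that owns each player's main HUD and relays game updates to it.
; On BeginPlay it creates W_MainHUD for the local player, covering both the authority's own controller and remote clients.
; Public events for health, prop setup, win screen, countdown and crosshair hits forward to matching OnClient events that drive the widget.
; It stores IsProp at setup to pass into the win screen.
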(event `self.ReceiveBeginPlay`
  ;[1 1 1] Creating HUD for Client
  (`/Engine/EditorBlueprintResources/ActorMacros.Switch Has Authority`
    (:`Authority`
      (if (`self.IsLocalPlayerController`)
        (bind _returnvalue (`|CreateWidget` "/Game/Core/Widgets/W_MainHUD.W_MainHUD_C" self :!label _label))
        (bind _output_get (set `self.MainHUDRef` _returnvalue))
        (`UserWidget.AddToViewport` _output_get 0)))
    (:`Remote`
      (goto _label))))

(event `/Game/Core/Blueprint/Interfaces/BPI_PropHuntController.UpdateHealthWidget`
  (params (Health :type "Float (double-precision)"))
  (`self.UpdateHealthOnClient` Health))

(event `/Game/Core/Blueprint/Interfaces/BPI_PropHuntController.SetupPropWidget`
  (params (`isProp?` :type Boolean))
  (set `self.Is Prop?` `isProp?`)
  (`self.SetPropOnClient` `isProp?`))

(event `SetPropOnClient`
  (params (`is Prop?` :type Boolean))
  (`/Game/Core/Widgets/W_MainHUD.SetupPropWidegts` (`self.MainHUDRef`) `is Prop?`))

(event `UpdateHealthOnClient`
  (params (Health :type "Float (double-precision)"))
  (`/Game/Core/Widgets/W_MainHUD.UpdateHealthBar` (`self.MainHUDRef`) Health))

(event `/Game/Core/Blueprint/Interfaces/BPI_PropHuntController.ShowWinScreenWidget`
  (params (`PropWin?` :type Boolean))
  (`self.ShowWinScreenOnClient` `PropWin?` (`self.Is Prop?`)))

(event `ShowWinScreenOnClient`
  (params (`PropWon?` :type Boolean) (`IsProp?` :type Boolean))
  (`/Game/Core/Widgets/W_MainHUD.ShowWinScreen` (`self.MainHUDRef`) `PropWon?` `IsProp?`))

(event `/Game/Core/Blueprint/Interfaces/BPI_PropHuntController.StartCountDownWidget`
  (`self.StartCountDownOnClient`))

(event `StartCountDownOnClient`
  (`/Game/Core/Widgets/W_MainHUD.StartTimer` (`self.MainHUDRef`)))

(event `/Game/Core/Blueprint/Interfaces/BPI_PropHuntController.PlayCrossHairHit`
  (`self.ShowCrossHairHitOnClient`))

(event `ShowCrossHairHitOnClient`
  (`/Game/Core/Widgets/W_MainHUD.PlayHitAnimation` (`self.MainHUDRef`)))

(fn `UserConstructionScript`)